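; Game mode for an endless runner that lays down the ground track.
; On BeginPlay it spawns a set number of initial ground blocks by calling AddBlock repeatedly.
; AddBlock spawns a BP_GroundBlock end to end along the X axis, offset by block length times the running count, passes that count as the block's index, then increments it.
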(event `self.ReceiveBeginPlay`
  (for _ (range (`self.InitialBlockCount`))
    (`self.AddBlock`)))

(fn `AddBlock`
  (`|SpawnActorFromClass` "/Game/EndlessRunner/Ground/BP_GroundBlock.BP_GroundBlock_C" (`KismetMathLibrary.MakeTransform` (`KismetMathLibrary.MakeVector` (* (`self.BlockActorLength`) (`self.BlockCount`)))) "AlwaysSpawn" "OverrideRootScale" null (`self.BlockCount`) null)
  (`/Engine/EditorBlueprintResources/StandardMacros.IncrementInt` (`self.BlockCount`)))

(fn `UserConstructionScript`)