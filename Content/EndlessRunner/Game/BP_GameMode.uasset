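; Game mode for the endless runner that builds the starting track and handles pausing and game over.
; On BeginPlay it shows the cursor and spawns the initial ground blocks, with AddBlock placing each one end to end along X and passing its index.
; PauseGame toggles pause, input mode and a lazily created, reused pause menu widget.
; GameOver shows the game over widget, pauses and switches to UI-only input.
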(event `self.ReceiveBeginPlay`
  (bind _returnvalue (`GameplayStatics.GetPlayerController` 0))
  (set `PlayerController.bShowMouseCursor` true _returnvalue)
  (`WidgetBlueprintLibrary.SetInputMode_GameOnly` _returnvalue)
  (for _ (range (`self.InitialBlockCount`))
    (`self.AddBlock`)))

(fn `AddBlock`
  (`|SpawnActorFromClass` "/Game/EndlessRunner/Ground/BP_GroundBlock.BP_GroundBlock_C" (`KismetMathLibrary.MakeTransform` (`KismetMathLibrary.MakeVector` (* (`self.BlockActorLength`) (`self.BlockCount`)))) "AlwaysSpawn" "OverrideRootScale" null (`self.BlockCount`) null)
  (`/Engine/EditorBlueprintResources/StandardMacros.IncrementInt` (`self.BlockCount`)))

(fn `Game Over`
  (bind _returnvalue (`|CreateWidget` "/Game/EndlessRunner/UI/WBP_GameOver.WBP_GameOver_C"))
  (`UserWidget.AddToViewport` _returnvalue 0)
  (`GameplayStatics.SetGamePaused` true)
  (`WidgetBlueprintLibrary.SetInputMode_UIOnlyEx` (`GameplayStatics.GetPlayerController` 0) _returnvalue))

(fn `PauseGame`
  (bind _returnvalue (`GameplayStatics.GetPlayerController` 0))
  (bind _pausemenuwidget (`self.PauseMenuWidget`))
  (if (`self.bIsGamePaused`)
    (set `self.bIsGamePaused` false)
    (`WidgetBlueprintLibrary.SetInputMode_GameOnly` (`GameplayStatics.GetPlayerController` 0))
    (`GameplayStatics.SetGamePaused` false)
    (`/Engine/EditorBlueprintResources/StandardMacros.IsValid` (`self.PauseMenuWidget`)
      (:`Is Valid`
        (`Widget.SetVisibility` _pausemenuwidget "Collapsed")))
    (else
      (bind _output_get (set `self.bIsGamePaused` true))
      (`GameplayStatics.SetGamePaused` _output_get)
      (`/Engine/EditorBlueprintResources/StandardMacros.IsValid` (`self.PauseMenuWidget`)
        (:`Is Valid`
          (`Widget.SetVisibility` _pausemenuwidget "Visible"))
        (:`Is Not Valid`
          (bind _returnvalue_2 (`|CreateWidget` "/Game/EndlessRunner/UI/WBP_PauseMenu.WBP_PauseMenu_C" _returnvalue))
          (bind _output_get_2 (set `self.PauseMenuWidget` _returnvalue_2))
          (`UserWidget.AddToViewport` _output_get_2 0)))
      (`WidgetBlueprintLibrary.SetInputMode_UIOnlyEx` _returnvalue (`self.PauseMenuWidget`)))))

(fn `UserConstructionScript`)