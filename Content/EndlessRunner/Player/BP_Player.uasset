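; Player character for an endless runner that runs forward automatically at increasing speed, with lane switching, jumping and sliding.
; Input sets targets that Tick interpolates toward: lane Y from GameMode lane settings, and capsule half-height for slides.
; Obstacle hits grant brief immunity and shorten EnemySpringArm, with retriggerable delays resetting immunity and hit count.
; The game quits once that arm nearly reaches zero; Tick also prints its length.
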(event `self.ReceiveBeginPlay`
  (bind (_returnvalue_x _returnvalue_y) (`KismetMathLibrary.BreakVector` (`self.K2_GetActorLocation`)))
  (set `self.StartLocation` _returnvalue_y)
  (bind _asbp_game_mode (cast `/Game/EndlessRunner/GameModes/BP_GameMode` (`GameplayStatics.GetGameMode`)))
  (set `self.GameModeRef` _asbp_game_mode)
  (`self.SwitchLane` 0))

(event `self.ReceiveTick`
  (params (DeltaSeconds :type "Float (single-precision)"))
  (`self.AddMovementInput` (`self.GetActorForwardVector`))
  (`self.SetActorLocationInterp` DeltaSeconds)
  (`self.IncreaseWalkSpeed`)
  (`self.SetCapsuleHalfHeightInterp` DeltaSeconds)
  (`self.SetEnemySpringArmLengthInterp` DeltaSeconds)
  (set `self.bIsJumping` (`NavMovementComponent.IsFalling` (`self.CharacterMovement`)))
  (`KismetSystemLibrary.PrintString` (`KismetStringLibrary.Conv_DoubleToString` (`SpringArmComponent.TargetArmLength` (`self.EnemySpringArm`))) true true (struct :`G` 0.66 :`B` 1.0 :`A` 1.0) DeltaSeconds))

(event `InputAction|Jump`
  (params (Key :type "Key Structure"))
  (:`Pressed`
    (`self.Jump`)
    (`self.ResetSlide`)))

(event `InputAction|Move Left`
  (params (Key :type "Key Structure"))
  (:`Pressed`
    (`self.SwitchLane` -1)))

(event `InputAction|Move Right`
  (params (Key :type "Key Structure"))
  (:`Pressed`
    (`self.SwitchLane` 1)))

(event `InputAction|Slide`
  (params (Key :type "Key Structure"))
  (:`Pressed`
    (if (not (`self.bIsJumping`))
      (set `self.bIsSliding` true)
      (set `self.TargetCapsuleHalfHeight` (`self.SlideCapsuleHalfHeight`))
      (`KismetSystemLibrary.RetriggerableDelay` (`self.SlideDuration`))
      (`self.ResetSlide`))))

(event `ResetSlide`
  (set `self.bIsSliding` false)
  (set `self.TargetCapsuleHalfHeight` (`self.OrigCapsuleHalfHeight`)))

(event `OnObstacleOverlap`
  (params (Obstacle :type "/Game/EndlessRunner/Obstacles/BP_ObstacleBase Object Reference"))
  (if (not (`self.bIsImmune`))
    (`|ExecutionSequence`
      (:`then_0`
        (set `self.bIsImmune` true)
        (`KismetSystemLibrary.RetriggerableDelay` (`self.ImmuneDuration`))
        (`self.ResetImmune`))
      (:`then_1`
        (bind _result (`/Engine/EditorBlueprintResources/StandardMacros.IncrementInt` (`self.HitCount`))
          (:`  `
            (set `self.TargetEnemySpringArmLength` (* (`self.OrigEnemySpringArmLength`) (select `bool` (== _result 1) :`false` 0.0 :`true` 0.33)))
            (set `self.EnemySpringArmInterpSpeed` 10.0)
            (if (< (`self.HitCount`) (`self.MaxHits`))
              (`KismetSystemLibrary.RetriggerableDelay` (`self.HitResetDuration`))
              (`self.ResetHit`))))))))

(event `ResetHit`
  (set `self.HitCount` 0)
  (set `self.TargetEnemySpringArmLength` (`self.OrigEnemySpringArmLength`))
  (set `self.EnemySpringArmInterpSpeed` 2.0))

(event `ResetImmune`
  (set `self.bIsImmune` false))

(event `EndGame`
  (`KismetSystemLibrary.QuitGame` null "Quit"))

(fn `IncreaseWalkSpeed`
  (set `CharacterMovementComponent.MaxWalkSpeed` (`KismetMathLibrary.FClamp` (+ (`CharacterMovementComponent.MaxWalkSpeed` (`self.CharacterMovement`)) (`self.SpeedIncrease`)) 0.0 (`self.MaxSpeed`)) (`self.CharacterMovement`)))

(fn `SetActorLocationInterp`
  (params (DeltaTime :type "Float (double-precision)"))
  (bind (_returnvalue_x _returnvalue_y _returnvalue_z) (`KismetMathLibrary.BreakVector` (`self.K2_GetActorLocation`)))
  (`self.K2_SetActorLocation` (`KismetMathLibrary.MakeVector` _returnvalue_x (`KismetMathLibrary.FInterpTo` _returnvalue_y (`self.TargetLocation`) DeltaTime 10.0) _returnvalue_z)))

(fn `SetCapsuleHalfHeightInterp`
  (params (DeltaTime :type "Float (double-precision)"))
  (`CapsuleComponent.SetCapsuleHalfHeight` (`self.CapsuleComponent`) (`KismetMathLibrary.FInterpTo` (`CapsuleComponent.CapsuleHalfHeight` (`self.CapsuleComponent`)) (`self.TargetCapsuleHalfHeight`) DeltaTime 10.0) true))

(fn `SetEnemySpringArmLengthInterp`
  (params (DeltaTime :type "Float (double-precision)"))
  (bind _output_get (set `SpringArmComponent.TargetArmLength` (`KismetMathLibrary.FInterpTo` (`SpringArmComponent.TargetArmLength` (`self.EnemySpringArm`)) (`self.TargetEnemySpringArmLength`) DeltaTime (`self.EnemySpringArmInterpSpeed`)) (`self.EnemySpringArm`)))
  (if (< _output_get 10.0)
    (`self.EndGame`)))

(fn `SwitchLane`
  (params (Direction :type Integer))
  (set `self.CurrentLane` (`KismetMathLibrary.Clamp` (+ (`self.CurrentLane`) Direction) 0 (- (`/Game/EndlessRunner/GameModes/BP_GameMode.NumLanes` (`self.GameModeRef`)) 1)))
  (set `self.TargetLocation` (+ (`self.StartLocation`) (* (`/Game/EndlessRunner/GameModes/BP_GameMode.LaneWidth` (`self.GameModeRef`)) (`self.CurrentLane`)))))

(fn `UserConstructionScript`)