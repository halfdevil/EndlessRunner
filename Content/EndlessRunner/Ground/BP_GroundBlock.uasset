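; BP_GroundBlock is a ground segment for an endless runner, with a building on each side.
; On BeginPlay it gives the left and right buildings random meshes from BuildingMeshes.
; When BP_Player overlaps BlockCollision, it tells BP_GameMode to add a block, then destroys itself after a short delay.
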(event `self.ReceiveBeginPlay`
  (`StaticMeshComponent.SetStaticMesh` (`self.LeftBuilding`) (`KismetArrayLibrary.Array_Random` (`self.BuildingMeshes`)))
  (`StaticMeshComponent.SetStaticMesh` (`self.RightBuilding`) (`KismetArrayLibrary.Array_Random` (`self.BuildingMeshes`))))

(event `self.BlockCollision.OnComponentBeginOverlap`
  (params (OverlappedComponent :type "PrimitiveComponent Object Reference") (OtherActor :type "Actor Object Reference") (OtherComp :type "PrimitiveComponent Object Reference") (OtherBodyIndex :type Integer) (bFromSweep :type Boolean) (SweepResult :type "HitResult Structure (by ref)"))
  (cast `/Game/EndlessRunner/Player/BP_Player` OtherActor)
  (bind _asbp_game_mode (cast `/Game/EndlessRunner/GameModes/BP_GameMode` (`GameplayStatics.GetGameMode`)))
  (`/Game/EndlessRunner/GameModes/BP_GameMode.AddBlock` _asbp_game_mode)
  (`KismetSystemLibrary.Delay` 2.0)
  (`self.DestroyBlock`))

(event `DestroyBlock`
  (`self.K2_DestroyActor`))

(fn `UserConstructionScript`)